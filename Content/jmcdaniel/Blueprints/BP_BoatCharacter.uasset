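; Player boat character that circles its starting point on left/right input and pushes iceberg chunks with a "Staple" action.
; Tick advances an orbit angle, places the boat on that circle facing the center, and sets its height from WaterSettings wave deltas in FloatOnWater.
; A line trace toward the center targets Iceberg_chunk1 components, and Staple applies an inward impulse to the current target.
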(event EventBeginPlay
  (bind _capsulecomponent (Variables|Collision|GetCapsuleComponent))
  (bind _returnvalue (Transformation|GetWorldLocation _capsulecomponent))
  (Utilities|FlowControl|Sequence
    (:then_0
      (bind _outactors (Actor|GetAllActorsOfClass "/Game/PhysicalWaterSurface/Blueprints/WaterSettings.WaterSettings_C"))
      (Variables|Private|SetWaterSettings (Utilities|Array|Get(acopy) _outactors)))
    (:then_1
      (Variables|Private|SetInitialZ (.z _returnvalue)))
    (:then_2
      (bind _output_get (Variables|Private|SetStartLocation (Math|Vector|MakeVector (.x _returnvalue) (.y _returnvalue) (.z _returnvalue)))))))

(event EventTick
  (params (DeltaSeconds :type Float%20%28single-precision%29))
  (bind _returnvalue (Transformation|GetActorRotation))
  (bind _capsulecomponent (Variables|Collision|GetCapsuleComponent))
  (bind _startlocation (Variables|Private|GetStartLocation))
  (bind _returnvalue_2 (Transformation|GetWorldLocation _capsulecomponent))
  (Utilities|FlowControl|Sequence
    (:then_0
      (CallFunction|FloatonWater (Variables|Private|GetWaterSettings) (Variables|Private|GetInitialZ)))
    (:then_1
      (bind _output_get (Variables|Private|Set_currX (+ (* (Variables|Public|GetRadius) (Math|Trig|Sin(Degrees) (Variables|Private|Get_theta))) (.x _startlocation)))))
    (:then_2
      (if (Variables|Private|GetIsMovingLeft)
        (Variables|Private|Set_theta (+ (Variables|Private|Get_theta) (* -1 (Variables|Public|GetSpeed))))))
    (:then_3
      (if (Variables|Private|GetIsMovingRight)
        (Variables|Private|Set_theta (+ (Variables|Private|Get_theta) (Variables|Public|GetSpeed)))))
    (:then_4
      (bind _output_get_2 (Variables|Private|Set_currY (+ (* (Variables|Public|GetRadius) (Math|Trig|Cos(Degrees) (Variables|Private|Get_theta))) (.y _startlocation)))))
    (:then_5
      (Transformation|SetActorLocation (Math|Vector|MakeVector _output_get _output_get_2 (.z (Transformation|GetActorLocation))) false true))
    (:then_6
      (Development|PrintString (Utilities|String|Append "Ori: " (Utilities|String|ToString(Vector) _returnvalue_2)) true true "(R=0.000000,G=0.660000,B=1.000000,A=1.000000)" 0.0)
      (Transformation|SetWorldRotation (Variables|Collision|GetCapsuleComponent) (Math|Rotator|MakeRotator (.roll _returnvalue) (.pitch _returnvalue) (.yaw (Math|Rotator|FindLookatRotation _returnvalue_2 (Variables|Private|GetStartLocation)))) false false))
    (:then_7
      (bind _outhit (Collision|LineTraceByChannel (Transformation|GetActorLocation) (Variables|Private|GetStartLocation) "TraceTypeQuery1" false 0 "ForOneFrame"))
      (Utilities|Casting|CastToIceberg_chunk1 (Components|GetOwner (.hitcomponent _outhit))
        (:then
          (Variables|Default|SetTargetIcebergChunkComponent (.hitcomponent _outhit) :!label _label))
        (:CastFailed
          (Utilities|Casting|CastToIceberg_chunk1 (Components|GetOwner (.hitcomponent _outhit))
            (:then
              (goto _label))
            (:CastFailed
              (Utilities|Casting|CastToIceberg_chunk1 (Components|GetOwner (.hitcomponent _outhit))
                (:then
                  (goto _label))
                (:CastFailed
                  (Variables|Default|SetTargetIcebergChunkComponent 0))))))))))

(event Input|ActionEvents|InputActionStaple
  (params (Key :type Key%20Structure))
  (bind _targeticebergchunkcomponent (Variables|Default|GetTargetIcebergChunkComponent))
  (:Pressed
    (Utilities|IsValid _targeticebergchunkcomponent
      (:Is%20Valid
        (Development|PrintString "STAPLE!")
        (Physics|AddImpulse _targeticebergchunkcomponent (* (Math|Vector|GetUnitDirection(Vector) (Transformation|GetActorLocation) (Variables|Private|GetStartLocation)) (Variables|Public|GetImpulseStrength)) "None" false)))))

(event Input|ActionEvents|InputActionMoveLeft
  (params (Key :type Key%20Structure))
  ;[1 1 1] Character State / Input Handling
  (:Pressed
    (Variables|Private|SetIsMovingLeft true))
  (:Released
    (Variables|Private|SetIsMovingLeft false)))

(event Input|ActionEvents|InputActionMoveRight
  (params (Key :type Key%20Structure))
  ;[1 1 1] Character State / Input Handling
  (:Pressed
    (Variables|Private|SetIsMovingRight true))
  (:Released
    (Variables|Private|SetIsMovingRight false)))

(fn ConstructionScript)

(fn FloatonWater
  (params (WaterSettings :type Water%20Settings%20Object%20Reference) (InitialZ :type Float%20%28single-precision%29))
  (bind _returnvalue (Transformation|GetActorLocation))
  (Utilities|IsValid WaterSettings
    (:Is%20Valid
      (bind _delta (Default|CalculateDeltaOnly WaterSettings (Math|Vector2D|MakeVector2D (.x _returnvalue) (.y _returnvalue))))
      (Transformation|SetActorLocationAndRotation (Math|Vector|MakeVector 0.0 0.0 (+ (.z _delta) InitialZ)) "0, 0, 0"))))