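; Buoyancy component that floats its owning actor on the waves computed by WaterSettings.
; Single-point mode moves and tilts the actor directly with the surface.
; Auto (rectangle or ellipse grid) and manual point modes apply physics buoyancy forces by depth, plus damping, horizontal water drag and enter/leave events.
; To limit cost, it staggers wave queries across points and frames, extrapolating depth between updates and skipping actors high above water.
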(event Custom|HasLeftWater
  ;[1 1 1] An event is triggered when objects enter/leave the water
  (if (Variables|Default|GetDrawDebug)
    (Development|PrintString (Utilities|String|Append (Utilities|GetDisplayName self) " left the water"))))

(event Custom|HasEnteredWater
  ;[1 1 1] An event is triggered when objects enter/leave the water
  (if (Variables|Default|GetDrawDebug)
    (Development|PrintString (Utilities|String|Append (Utilities|GetDisplayName self) " entered the water"))))

(event EventTick
  (params (DeltaSeconds :type Float%20%28single-precision%29))
  (bind _returnvalue (Utilities|Time|GetWorldDeltaSeconds))
  (bind _initiallocation_global_ (Variables|Default|GetInitialLocation%28global%29))
  (bind _initiallocation_global__2 (Variables|Default|GetInitialLocation%28global%29))
  (bind _pointsdepth (Variables|Default|GetPointsDepth))
  (bind _primcomponent (Variables|Default|GetPrimComponent))
  (bind _watersettings (Variables|Default|GetWaterSettings))
  (bind _deltaprev (Variables|Default|GetDeltaPrev))
  (bind _deltaprevprev (Variables|Default|GetDeltaPrevPrev))
  (bind _returnvalue_2 (Math|Vector|GetVectorArrayAverage _deltaprevprev))
  (bind _returnvalue_3 (Math|Vector|GetVectorArrayAverage _deltaprev))
  (bind _maxvalue (Math|Float|MaxOfFloatArray _pointsdepth))
  (bind _returnvalue_4 (|((({843D29D5-48C7-E573-2F81-21B612EF48D7}+1)*(dT*{2321D17E-42B6-057B-8412-7394C824EBD0}))/{2245F6F2-408D-474D-88DE-DCB1CAB9877A}) _returnvalue))
  (bind _returnvalue_5 (- _returnvalue_2 _returnvalue_3))
  (bind _returnvalue_6 (> _maxvalue 0.0))
  (bind _returnvalue_7 (/ _returnvalue_5 _returnvalue_4))
  ;[1 1 1] Each Tick we update the buoyancy calculation
  (if (Variables|Default|GetEnableBuoyancy)
    (switch Utilities|FlowControl|Switch|SwitchonBuoyancyModes (Variables|Default|GetBuoyancyMode)
      (:NewEnumerator2
        ;[1 0.42 0.4229] SinglePoint buoyancy mode
        ;;[1 1 1] calculate delta and normal
        (bind (_delta _normal) (Default|CalculateDeltaNormal (Variables|Default|GetWaterSettings) (Math|Vector2D|MakeVector2D (.x _initiallocation_global_) (.y _initiallocation_global_))))
        (Transformation|SetActorLocationAndRotation (Variables|Default|GetOwner) (+ _delta (Math|Vector|MakeVector (.x _initiallocation_global__2) (.y _initiallocation_global__2) (Variables|/Game/PhysicalWaterSurface/Blueprints/WaterSettings.WaterSettings_C|GetSeaLevel (Variables|Default|GetWaterSettings)))) (Math|Rotator|CombineRotators (Variables|Default|GetInitialRotation) (CallFunction|RotatorfromNormal _normal))))
      (:NewEnumerator1
        ;[1 1 1] if far above water, dont execute
        (if (|(ActorZ<((SeaLevel+{A57CC1D5-46F8-A1FB-B9C5-2498A4F55B50})+{897E28A4-4893-1FDC-27C3-90940C7E0ED9})) (.z (Transformation|GetActorLocation (Variables|Default|GetOwner))) (Variables|/Game/PhysicalWaterSurface/Blueprints/WaterSettings.WaterSettings_C|GetSeaLevel (Variables|Default|GetWaterSettings))) :!label _label
          (Utilities|FlowControl|Sequence
            (:then_0
              ;[0.4549 0.7216 1] Advanced Buoyancy mode
              (Utilities|FlowControl|Sequence
                (:then_0
                  ;;[1 1 1] fill PointsIdxToCalculate array
                  (Variables|Default|SetPointsCalculated 0)
                  (Variables|Default|SetActorTransform (Transformation|GetWorldTransform (Variables|Default|GetPrimComponent)))
                  (|FindPointsIdxToCalculate))
                (:then_1
                  ;;[1 1 1] for all points...
                  (for (_array_element _array_index) (Variables|Default|GetPoints)
                    (Variables|Default|SetArrayElem _array_element)
                    (Variables|Default|SetArrayIdx _array_index)
                    (Utilities|FlowControl|Sequence
                      (:then_0
                        ;;[1 1 1] PointsLocationPrev stores the locations fom the last frame
                        (Utilities|TransferVecArrayElem (Variables|Default|GetPointsLocation) (Variables|Default|GetPointsLocationPrev) (Variables|Default|GetArrayIdx) true
                          (:Done
                            ;;[1 1 1] PointsLocation store the current coordinates of all points in local frame
                            (Utilities|Array|SetArrayElem (Variables|Default|GetPointsLocation) (Variables|Default|GetArrayIdx) (Math|Transform|TransformLocation (Variables|Default|GetActorTransform) (Variables|Default|GetArrayElem)) true))))
                      (:then_1
                        ;;[1 1 1] update this point?
                        (if (or (Utilities|Array|ContainsItem (Variables|Default|GetPointsIdxToCalculate) (Variables|Default|GetArrayIdx)) (not (Utilities|Array|Get(acopy) (Variables|Default|GetPointInitialized) (Variables|Default|GetArrayIdx))))
                          ;;[1 1 1] calculate depth and new relative speed
                          ;;
                          ;; This is a recursive algorithm.
                          ;; DeltaPrev is the Delta value from the last frame.
                          ;; It is used as an estimate in the current frame for the input to the call of CalculateDeltaOnly.
                          (Utilities|TransferVecArrayElem (Variables|Default|GetDeltaPrev) (Variables|Default|GetDeltaPrevPrev) (Variables|Default|GetArrayIdx) true ; save previous Delta value
                            (:Done
                              (bind _delta_2 (Default|CalculateDeltaOnly _watersettings (+ (Math|Vector2D|MakeVector2D (.x (Utilities|Array|Get(acopy) (Variables|Default|GetPointsLocation) (Variables|Default|GetArrayIdx))) (.y (Utilities|Array|Get(acopy) (Variables|Default|GetPointsLocation) (Variables|Default|GetArrayIdx)))) (Math|Vector2D|MakeVector2D (.x (Utilities|Array|Get(acopy) (Variables|Default|GetDeltaPrev) (Variables|Default|GetArrayIdx))) (.y (Utilities|Array|Get(acopy) (Variables|Default|GetDeltaPrev) (Variables|Default|GetArrayIdx))))))) ; calculate displacement vector of water surface that ends at the point\ncalling this function is quite expensive
                              (Utilities|Array|SetArrayElem (Variables|Default|GetDeltaPrev) (Variables|Default|GetArrayIdx) (Math|Vector|NegateVector _delta_2) true) ; save Delta
                              (Utilities|Array|SetArrayElem (Variables|Default|GetPointsDepth) (Variables|Default|GetArrayIdx) (- (+ (.Z (Math|Vector|BreakVector _delta_2)) (Variables|/Game/PhysicalWaterSurface/Blueprints/WaterSettings.WaterSettings_C|GetSeaLevel _watersettings)) (.z (Utilities|Array|Get(acopy) (Variables|Default|GetPointsLocation) (Variables|Default|GetArrayIdx)))) true) ; save depth of this point\nbelow the surface
                              ;;;[1 1 1] prevent 0/0 log message
                              (if (!= (Utilities|Array|Get(acopy) (Variables|Default|GetPointsUpdateCumTime) (Variables|Default|GetArrayIdx)) 0.0)
                                (Utilities|Array|SetArrayElem (Variables|Default|GetPointsSurfaceSpeed) (Variables|Default|GetArrayIdx) (|((h1-h0)/dt) (+ (.Z (Math|Vector|BreakVector _delta_2)) (Variables|/Game/PhysicalWaterSurface/Blueprints/WaterSettings.WaterSettings_C|GetSeaLevel _watersettings)) (Utilities|Array|Get(acopy) (Variables|Default|GetPointsWaveHeight) (Variables|Default|GetArrayIdx)) (Utilities|Array|Get(acopy) (Variables|Default|GetPointsUpdateCumTime) (Variables|Default|GetArrayIdx))) true) ; save vertical speed of the\nwater surface at this point
                              )
                              (Utilities|Array|SetArrayElem (Variables|Default|GetPointsWaveHeight) (Variables|Default|GetArrayIdx) (+ (.Z (Math|Vector|BreakVector _delta_2)) (Variables|/Game/PhysicalWaterSurface/Blueprints/WaterSettings.WaterSettings_C|GetSeaLevel _watersettings)) true) ; dont do this earlier!
                              (Utilities|Array|SetArrayElem (Variables|Default|GetPointsUpdateCumTime) (Variables|Default|GetArrayIdx) 0.0 true)
                              ;;;[1 1 1] mark this point as initialized
                              (Utilities|Array|SetArrayElem (Variables|Default|GetPointInitialized) (Variables|Default|GetArrayIdx) true true)))
                          (else
                            ;;[1 1 1] extrapolate depth using the last known speed
                            (Utilities|AddtoArrayElem (Variables|Default|GetPointsUpdateCumTime) (Variables|Default|GetArrayIdx) (Utilities|Time|GetWorldDeltaSeconds)
                              (:Ecec
                                (Utilities|Array|SetArrayElem (Variables|Default|GetPointsDepth) (Variables|Default|GetArrayIdx) (|((DepthPrev+(dt*vSurf))-(PtHeight-PtHeightPrev)) (Utilities|Array|Get(acopy) (Variables|Default|GetPointsDepth) (Variables|Default|GetArrayIdx)) (Utilities|Time|GetWorldDeltaSeconds) (Utilities|Array|Get(acopy) (Variables|Default|GetPointsSurfaceSpeed) (Variables|Default|GetArrayIdx)) (.z (Utilities|Array|Get(acopy) (Variables|Default|GetPointsLocation) (Variables|Default|GetArrayIdx))) (.z (Utilities|Array|Get(acopy) (Variables|Default|GetPointsLocationPrev) (Variables|Default|GetArrayIdx)))) true)))))))))))
            (:then_1
              ;[0.4549 0.7216 1] add forces and damping
              (Utilities|FlowControl|Sequence
                (:then_0
                  ;;[1 1 1] Trigger events when entering/leaving the water
                  (if (and (not (Variables|Default|GetbAnySubmerged)) _returnvalue_6)
                    (CallFunction|HasEnteredWater)
                    (elif (and (Variables|Default|GetbAnySubmerged) (not _returnvalue_6))
                      (CallFunction|HasLeftWater)))
                  (Variables|Default|SetbAnySubmerged _returnvalue_6))
                (:then_1
                  ;;[1 1 1] Add force for all PointsDepth values
                  (for (_array_element_2 _array_index_2) (Variables|Default|GetPointsDepth)
                    (Variables|Default|SetPtLoc (Utilities|Array|Get(acopy) (Variables|Default|GetPointsLocation) _array_index_2))
                    (if (> _array_element_2 0.0)
                      (Class|PrimitiveComponent|AddForceatLocation (Variables|Default|GetPrimComponent) (Math|Vector|MakeVector 0.0 0.0 (|(({73F4D735-4DB2-0E87-B90B-FF95A3B3027E}*((Depth/{A57CC1D5-46F8-A1FB-B9C5-2498A4F55B50})*({6F289B36-4AAF-C80D-6F6D-77BA0FA3074C}*981)))/{2321D17E-42B6-057B-8412-7394C824EBD0}) _array_element_2)) (Variables|Default|GetPtLoc) "None"))
                    ;;;[1 1 1] draw debug objects
                    (if (Variables|Default|GetDrawDebug)
                      (Rendering|Debug|DrawDebugSphere (Variables|Default|GetPtLoc) 5.0 12 "(R=1.000000,G=0.000000,B=0.000000,A=1.000000)" 0.0)
                      (if (> (* (|(({73F4D735-4DB2-0E87-B90B-FF95A3B3027E}*((Depth/{A57CC1D5-46F8-A1FB-B9C5-2498A4F55B50})*({6F289B36-4AAF-C80D-6F6D-77BA0FA3074C}*981)))/{2321D17E-42B6-057B-8412-7394C824EBD0}) _array_element_2) 0.003) 0.0)
                        (Rendering|Debug|DrawDebugArrow (Variables|Default|GetPtLoc) (+ (Variables|Default|GetPtLoc) (Math|Vector|MakeVector 0.0 0.0 (* (|(({73F4D735-4DB2-0E87-B90B-FF95A3B3027E}*((Depth/{A57CC1D5-46F8-A1FB-B9C5-2498A4F55B50})*({6F289B36-4AAF-C80D-6F6D-77BA0FA3074C}*981)))/{2321D17E-42B6-057B-8412-7394C824EBD0}) _array_element_2) 0.003))) 1e+02 "(R=1.000000,G=0.000000,B=0.000000,A=1.000000)" 0.0 0.0)))))
                (:then_2
                  ;;[1 1 1] increase damping if submerged in water
                  (Class|PrimitiveComponent|SetLinearDamping _primcomponent (Math|Float|SelectFloat (Variables|Default|GetLinearDamping) 0.0 (Variables|Default|GetbAnySubmerged)))
                  (Class|PrimitiveComponent|SetAngularDamping _primcomponent (Math|Float|SelectFloat (Variables|Default|GetAngularDamping) 0.0 (Variables|Default|GetbAnySubmerged))))
                (:then_3
                  ;;[1 1 1] add lateral drag force from horizontal water motion
                  (if (and (Variables|Default|GetbAnySubmerged) (Math|Vector|NotEqual(Vector) _returnvalue_2 "0, 0, 0" 0.0001))
                    (bind _returnvalue_8 (Physics|GetPhysicsLinearVelocity (Variables|Default|GetPrimComponent) "None")) ; own speed
                    (Class|PrimitiveComponent|AddForceatLocation (Variables|Default|GetPrimComponent) (Math|Vector|MakeVector (.x (* (- (Math|Vector2D|MakeVector2D (.x _returnvalue_7) (.y _returnvalue_7)) (Math|Vector2D|MakeVector2D (.x _returnvalue_8) (.y _returnvalue_8))) (* (Variables|Default|GetDragMultiplier) (Variables|Default|GetMass)))) (.y (* (- (Math|Vector2D|MakeVector2D (.x _returnvalue_7) (.y _returnvalue_7)) (Math|Vector2D|MakeVector2D (.x _returnvalue_8) (.y _returnvalue_8))) (* (Variables|Default|GetDragMultiplier) (Variables|Default|GetMass)))) 0.0) (Physics|GetCenterOfMass (Variables|Default|GetPrimComponent) "None") "None"))))))
          (else
            ;[1 1 1] buoyancy is not active because object is high above water
            (if (Variables|Default|GetDrawDebug)
              (Development|PrintString "high above water" true true "(R=0.000000,G=0.660000,B=1.000000,A=1.000000)" 0.1)))))
      (:NewEnumerator3
        (goto _label)))))

(event EventBeginPlay
  ;[1 1 1] Event Begin Play
  (Utilities|FlowControl|Sequence
    (:then_0
      ;[1 1 1] get reference to WaterSettings
      (bind _outactors (Actor|GetAllActorsOfClass "/Game/PhysicalWaterSurface/Blueprints/WaterSettings.WaterSettings_C"))
      (Variables|Default|SetWaterSettings (Utilities|Array|Get(acopy) _outactors)))
    (:then_1
      ;[1 1 1] get owner and his primitive component
      (Variables|Default|SetOwner (Components|GetOwner))
      (bind _asprimitive_component (Utilities|Casting|CastToPrimitiveComponent (VehicleSound|GetRootComponent (Variables|Default|GetOwner)))
        (:then
          (Variables|Default|SetPrimComponent _asprimitive_component))
        (:CastFailed
          (if (Utilities|Enum|NotEqual(Enum) (Variables|Default|GetBuoyancyMode) "NewEnumerator2") ; PrimComponent is not used in SinglePoint mode
            (Development|PrintString "RootComponent needs to be a PrimitiveComponent")))))
    (:then_2
      ;[1 1 1] Set Simulate Physics
      (if (Utilities|Enum|NotEqual(Enum) (Variables|Default|GetBuoyancyMode) "NewEnumerator2")
        (bind _asprimitive_component_2 (Utilities|Casting|CastToPrimitiveComponent (VehicleSound|GetRootComponent (Variables|Default|GetOwner))))
        (Physics|SetSimulatePhysics _asprimitive_component_2 true)
        ;[1 1 1] Set Mass
        (Variables|Default|SetMass (Physics|GetMass _asprimitive_component_2))))
    (:then_3
      ;[1 1 1] save initial location (global) and center of mass (local) and initial rotation
      (Variables|Default|SetInitialLocation%28global%29 (Transformation|GetActorLocation (Variables|Default|GetOwner)))
      (Variables|Default|SetInitialRotation (Transformation|GetActorRotation (Variables|Default|GetOwner))))
    (:then_4
      ;[1 1 1] find out actor dimensions
      (bind _dimensions (CallFunction|MeshDimensions (Variables|Default|GetOwner)))
      (bind _output_get (Variables|Default|SetActorDimensions _dimensions))
      (Variables|Default|SetActorHeight (.z _output_get)))
    (:then_5
      ;[1 1 1] Generate Auto Points Array
      (switch Utilities|FlowControl|Switch|SwitchonBuoyancyModes (Variables|Default|GetBuoyancyMode)
        (:NewEnumerator1
          (switch Utilities|FlowControl|Switch|SwitchonHullShapes (Variables|Default|GetPointsShape)
            (:NewEnumerator0
              (CallFunction|GenRectangularPoints))
            (:NewEnumerator2
              (CallFunction|GenCircPts))))
        (:NewEnumerator3
          _))
      ;;[1 1 1] calculate maximum possible amplitude
      (bind _sum (Utilities|Sum (Variables|/Game/PhysicalWaterSurface/Blueprints/WaterSettings.WaterSettings_C|GetA (Variables|Default|GetWaterSettings)))
        (:Done
          (Variables|Default|SetMaxAmplitude (* _sum 1e+02))
          ;;[1 1 1] determine number of points
          (Variables|Default|SetnPoints (Utilities|Array|Length (Variables|Default|GetPoints)))
          ;[1 1 1] Initialize the Array PointInitialized, set all elements to false
          (for (_ _array_index) (Variables|Default|GetPoints)
            (Utilities|Array|SetArrayElem (Variables|Default|GetPointInitialized) _array_index false true)))))
    (:then_6
      ;[1 1 1] without this, all instances would calculate on the same frame
      (Variables|Default|SetnPausedFrames (Math|Random|RandomIntegerinRange 0 (Variables|Default|GetnFramesPause))))))

(fn RotatorfromNormal
  (params (Normal :type Vector))
  (bind _returnvalue (Math|Vector|Normalize Normal))
  (bind _returnvalue_2 (Math|Vector|CrossProduct _returnvalue "0, 0,-1.000000"))
  ;[1 1 1] generate a rotator from a vector
  (return (Math|Vector|RotatorfromAxisandAngle _returnvalue_2 (Class|KismetMathLibrary|DegAsin (Math|Vector|VectorLength _returnvalue_2)))))

(fn MeshDimensions
  (params (self2 :type Actor%20Object%20Reference))
  ;[1 1 1] calculate min and max dimension of a mesh
  (LocalVariables|SetSelf%202%20loc self2)
  (Utilities|FlowControl|Sequence
    (:then_0
      ;[1 1 1] initialize to 0
      (LocalVariables|SetMinDim "0, 0, 0")
      (LocalVariables|SetMaxDim "0, 0, 0"))
    (:then_1
      ;[1 1 1] handle static mesh components
      (for _array_element (Actor|GetComponentsByClass (LocalVariables|GetSelf%202%20loc) "/Script/Engine.StaticMeshComponent")
        ;;[1 1 1] find absolute min/max
        (LocalVariables|SetMinDim (Math|Vector|MakeVector (Math|Float|Min(Float) (.x (.Min (Components|StaticMesh|GetLocalBounds _array_element))) (.x (LocalVariables|GetMinDim))) (Math|Float|Min(Float) (.y (.Min (Components|StaticMesh|GetLocalBounds _array_element))) (.y (LocalVariables|GetMinDim))) (Math|Float|Min(Float) (.z (.Min (Components|StaticMesh|GetLocalBounds _array_element))) (.z (LocalVariables|GetMinDim)))))
        (LocalVariables|SetMaxDim (Math|Vector|MakeVector (Math|Float|Max(Float) (.x (.Max (Components|StaticMesh|GetLocalBounds _array_element))) (.x (LocalVariables|GetMaxDim))) (Math|Float|Max(Float) (.y (.Max (Components|StaticMesh|GetLocalBounds _array_element))) (.y (LocalVariables|GetMaxDim))) (Math|Float|Max(Float) (.z (.Max (Components|StaticMesh|GetLocalBounds _array_element))) (.z (LocalVariables|GetMaxDim)))))))
    (:then_2
      ;[1 1 1] handle skeletal mesh components
      (for _array_element_2 (Actor|GetComponentsByClass (LocalVariables|GetSelf%202%20loc) "/Script/Engine.SkeletalMeshComponent")
        ;;[1 1 1] find absolute min/max
        (LocalVariables|SetMinDim (Math|Vector|MakeVector (Math|Float|Min(Float) (.x (LocalVariables|GetMinDim)) (.x (/ (Math|Vector|NegateVector (.BoxExtent (Collision|GetComponentBounds _array_element_2))) 2.0))) (Math|Float|Min(Float) (.y (LocalVariables|GetMinDim)) (.y (/ (Math|Vector|NegateVector (.BoxExtent (Collision|GetComponentBounds _array_element_2))) 2.0))) (Math|Float|Min(Float) (.z (LocalVariables|GetMinDim)) (.z (/ (Math|Vector|NegateVector (.BoxExtent (Collision|GetComponentBounds _array_element_2))) 2.0)))))
        (LocalVariables|SetMaxDim (Math|Vector|MakeVector (Math|Float|Max(Float) (.x (LocalVariables|GetMaxDim)) (.x (/ (.BoxExtent (Collision|GetComponentBounds _array_element_2)) 2.0))) (Math|Float|Max(Float) (.y (LocalVariables|GetMaxDim)) (.y (/ (.BoxExtent (Collision|GetComponentBounds _array_element_2)) 2.0))) (Math|Float|Max(Float) (.z (LocalVariables|GetMaxDim)) (.z (/ (.BoxExtent (Collision|GetComponentBounds _array_element_2)) 2.0)))))))
    (:then_3
      (return (- (LocalVariables|GetMaxDim) (LocalVariables|GetMinDim))))))

(fn GenRectangularPoints
  (bind _pointsoffset (Variables|Default|GetPointsOffset))
  (bind _actordimensions (Variables|Default|GetActorDimensions))
  ;[1 1 1] start point is at the corner
  ; increment depends on number of points
  (LocalVariables|SetX_Increment (|(Extent/({62823A3F-42DE-EF6F-2109-929C648AE4F0}-1)) (.x _actordimensions)))
  (LocalVariables|SetX_Start (* (.x _actordimensions) -0.5))
  (LocalVariables|SetY_Start (* (.y _actordimensions) -0.5))
  (LocalVariables|SetY_Increment (|(Extent/({9EE00E6E-48F9-C24A-F2D0-879506D2CFDA}-1)) (.y _actordimensions)))
  ;[1 1 1] x direction
  (for _index (range 0 (- (Variables|Default|GetnPointsX) 1))
    ;[1 1 1] y direction
    (for _index_2 (range 0 (- (Variables|Default|GetnPointsY) 1))
      ;[1 1 1] store points in array
      (Utilities|Array|Add (Variables|Default|GetPoints) (+ (* (Math|Vector|MakeVector (|({2395B32A-4876-65ED-E89B-C8ADE1F80E3F}+(idxX*{02A9F5FF-46B1-74EA-BFD6-139D45CD3E5F})) (Math|Conversions|ToFloat(Integer) _index)) (|({FEE2C461-4392-3B69-FAF6-3599E8F900CA}+(idxY*{4A6CBA40-43AA-5467-AE91-86976BC4AC8D})) (Math|Conversions|ToFloat(Integer) _index_2)) (Variables|Default|GetFloatHeight)) (Variables|Default|GetPointsScale)) (Math|Vector|MakeVector (.x _pointsoffset) (.y _pointsoffset) 0.0)))))
  ;[1 1 1] make sure the points will be updated randomly
  (Utilities|Array|Shuffle (Variables|Default|GetPoints))
  (return))

(fn GenCircPts
  (bind _pointsoffset (Variables|Default|GetPointsOffset))
  (bind _actordimensions (Variables|Default|GetActorDimensions))
  ;[1 1 1] calculate radial increment
  ; can be different for X and Y so that we get an oval shape
  (LocalVariables|SetRx_Increment (/ (/ (.x _actordimensions) 2.0) (Math|Conversions|ToFloat(Integer) (Variables|Default|GetnPointsX))))
  (LocalVariables|SetRy_Increment (/ (/ (.y _actordimensions) 2.0) (Math|Conversions|ToFloat(Integer) (Variables|Default|GetnPointsX))))
  ;[1 1 1] calculate angular increment
  (LocalVariables|SetPhi_Increment (/ (Math|Float|MultiplybyPi 2.0) (Math|Conversions|ToFloat(Integer) (Variables|Default|GetnPointsY))))
  ;[1 1 1] middle point
  (Utilities|Array|Add (Variables|Default|GetPoints) "0, 0, 0")
  ;[1 1 1] radial direction
  (for _index (range 1 (Variables|Default|GetnPointsX))
    ;[1 1 1] angular direction
    (for _index_2 (range 0 (- (Variables|Default|GetnPointsY) 1))
      ;[1 1 1] store points in array
      (Utilities|Array|Add (Variables|Default|GetPoints) (+ (* (Math|Vector|MakeVector (.X (Utilities|PolartoCartesian (|(nR*R_Increment) (Math|Conversions|ToFloat(Integer) _index) (Math|Float|Lerp (LocalVariables|GetRy_Increment) (LocalVariables|GetRx_Increment) (|((0.500000*(cos((2*x))))+0.500000) (|(nPhi*{3C902C39-4413-9478-8E50-89A30775620F}) (Math|Conversions|ToFloat(Integer) _index_2))))) (|(nPhi*{3C902C39-4413-9478-8E50-89A30775620F}) (Math|Conversions|ToFloat(Integer) _index_2)))) (.Y (Utilities|PolartoCartesian (|(nR*R_Increment) (Math|Conversions|ToFloat(Integer) _index) (Math|Float|Lerp (LocalVariables|GetRy_Increment) (LocalVariables|GetRx_Increment) (|((0.500000*(cos((2*x))))+0.500000) (|(nPhi*{3C902C39-4413-9478-8E50-89A30775620F}) (Math|Conversions|ToFloat(Integer) _index_2))))) (|(nPhi*{3C902C39-4413-9478-8E50-89A30775620F}) (Math|Conversions|ToFloat(Integer) _index_2)))) (Variables|Default|GetFloatHeight)) (Variables|Default|GetPointsScale)) (Math|Vector|MakeVector (.x _pointsoffset) (.y _pointsoffset) 0.0))))))