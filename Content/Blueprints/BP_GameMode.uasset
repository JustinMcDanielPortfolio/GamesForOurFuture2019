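; Game mode for a timed boat game where two tagged icebergs, a bear's and a human's, decide the outcome.
; BeginPlay finds both icebergs, starts a three-minute end timer plus looping one-second countdown and count-up timers, and creates the HUD, updated every tick.
; On timeout, whether each iceberg still has ice chunks picks one of four paused end screens.
; AddStaple tallies staples fired on the HUD.
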(event Custom|End%20Game
  (CallFunction|FindEnding))

(event EventBeginPlay
  (bind _outactors (Actor|GetAllActorsOfClass "/Game/Blueprints/Character/BP_BoatCharacter.BP_BoatCharacter_C"))
  (Variables|Default|SetTPC (Utilities|Array|Get(acopy) _outactors))
  (bind _iceberg (CallFunction|FindIcebergbyTag "Iceberg_Bear"))
  (Variables|Default|SetIceberg_Bear _iceberg)
  (bind _iceberg_2 (CallFunction|FindIcebergbyTag "Iceberg_Human"))
  (Variables|Default|SetIceberg_Human _iceberg_2)
  (Utilities|Time|SetTimerbyEvent (delegate Custom|End%20Game) 1.8e+02)
  (Utilities|Time|SetTimerbyFunctionName 0 "Set Global Time" 1.0 true)
  (Utilities|Time|SetTimerbyFunctionName 0 "Set Global Count Up" 1.0 true)
  (bind _returnvalue (Game|ConstructObjectfromClass "/Game/Blueprints/UI/WBP_HUD.WBP_HUD_C" (Game|GetPlayerController 0)))
  (bind _output_get (Variables|Default|SetWBP_HUDRef _returnvalue))
  (UserInterface|Viewport|AddtoViewport _output_get 0)
  (Variables|/Game/Blueprints/UI/WBP_HUD.WBP_HUD_C|SetSecondsRemaining (Variables|Default|GetWBP_HUDRef) (Math|Conversions|ToFloat(Integer) (Variables|Default|GetGlobal%20Time))))

(event EventTick
  (params (DeltaSeconds :type Float%20%28single-precision%29))
  (Variables|/Game/Blueprints/UI/WBP_HUD.WBP_HUD_C|SetSecondsRemaining (Variables|Default|GetWBP_HUDRef) (Math|Conversions|ToFloat(Integer) (Variables|Default|GetGlobal%20Time))))

(fn ConstructionScript)

(fn SetGlobalTime
  (bind _output_get (Variables|Default|SetGlobal%20Time (- (Variables|Default|GetGlobal%20Time) 1))))

(fn FindEnding
  (bind _tpc (Variables|Default|GetTPC))
  (Variables|Default|SetIs%20Human%20Alive? (> (Utilities|Array|Length (Variables|/Game/Blueprints/Iceberg_blueprints/Iceberg.Iceberg_C|GetIce_Chunks (Variables|Default|GetIceberg_Human))) 0))
  (Variables|Default|SetIs%20Bear%20Alive? (> (Utilities|Array|Length (Variables|/Game/Blueprints/Iceberg_blueprints/Iceberg.Iceberg_C|GetIce_Chunks (Variables|Default|GetIceberg_Bear))) 0))
  (if (Variables|Default|GetIs%20Human%20Alive?)
    (if (Variables|Default|GetIs%20Bear%20Alive?)
      (CallFunction|ShowBestWinScreen _tpc)
      (else
        (CallFunction|ShowHumanWinScreen _tpc)))
    (elif (Variables|Default|GetIs%20Bear%20Alive?)
      (CallFunction|ShowBearWinScreen _tpc)
      (else
        (CallFunction|ShowLoseScreen _tpc)))))

(fn ShowBestWinScreen
  (params (TPC :type Actor%20Object%20Reference))
  (Game|SetGamePaused true)
  (bind _returnvalue (UserInterface|CreateWidget "/Game/Blueprints/UI/Win_Screen.Win_Screen_C" (Game|GetPlayerController 0)))
  (UserInterface|Viewport|AddtoViewport _returnvalue 0))

(fn ShowHumanWinScreen
  (params (TPC :type Actor%20Object%20Reference))
  (Game|SetGamePaused true)
  (bind _returnvalue (UserInterface|CreateWidget "/Game/Blueprints/UI/Human_Win_Screen.Human_Win_Screen_C" (Game|GetPlayerController 0)))
  (UserInterface|Viewport|AddtoViewport _returnvalue 0))

(fn ShowBearWinScreen
  (params (TPC :type Actor%20Object%20Reference))
  (Game|SetGamePaused true)
  (bind _returnvalue (UserInterface|CreateWidget "/Game/Blueprints/UI/Bear_Win_Screen.Bear_Win_Screen_C" (Game|GetPlayerController 0)))
  (UserInterface|Viewport|AddtoViewport _returnvalue 0))

(fn ShowLoseScreen
  (params (TPC :type Actor%20Object%20Reference))
  (Game|SetGamePaused true)
  (bind _returnvalue (UserInterface|CreateWidget "/Game/Blueprints/UI/Lose_Screen.Lose_Screen_C" (Game|GetPlayerController 0)))
  (UserInterface|Viewport|AddtoViewport _returnvalue 0))

(fn SetGlobalCountUp
  (Variables|Default|SetGlobel%20Counter (+ (Variables|Default|GetGlobel%20Counter) 1)))

(fn FindIcebergbyTag
  (params (Tag :type Name))
  ;[1 1 1] Returns the first object that succeeds a cast to type "Iceberg" with matching Tag; returns NONE if not found.
  (bind _outactors (Actor|GetAllActorswithTag Tag))
  (for _array_element _outactors
    (bind _asiceberg (Utilities|Casting|CastToIceberg _array_element))
    (return _asiceberg))
  (return _asiceberg))

(fn AddStaple
  (bind _output_get (Variables|Default|SetStaplesFired (+ (Variables|Default|GetStaplesFired) 1)))
  (Variables|/Game/Blueprints/UI/WBP_HUD.WBP_HUD_C|SetStaplesUsed (Variables|Default|GetWBP_HUDRef) _output_get))