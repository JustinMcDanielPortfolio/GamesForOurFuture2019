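; Player boat character that circles its start point on left/right input and fires staples at iceberg chunks.
; Each tick it bobs via WaterSettings wave deltas, moves along a sine/cosine orbit, yaws toward the center and line-traces inward to target an uncaptured Iceberg_chunk1.
; Firing spawns a staple projectile, immediately marks any target stapled and impulses it forward.
; A self-rescheduling timer plays random paddle sound pairs.
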(event Custom|PlayBearSound
  (bind _nexttime (CallFunction|PlayPaddleSounds))
  (Utilities|Time|SetTimerbyEvent (delegate Custom|PlayBearSound) _nexttime))

(event EventBeginPlay
  (bind _capsulecomponent (Variables|Collision|GetCapsuleComponent))
  (bind _returnvalue (Transformation|GetWorldLocation _capsulecomponent))
  (Utilities|FlowControl|Sequence
    (:then_0
      (bind _outactors (Actor|GetAllActorsOfClass "/Game/PhysicalWaterSurface/Blueprints/WaterSettings.WaterSettings_C"))
      (Variables|Private|SetWaterSettings (Utilities|Array|Get(acopy) _outactors)))
    (:then_1
      (Variables|Private|SetInitialZ (.z _returnvalue)))
    (:then_2
      (Variables|Private|SetStartLocation (Math|Vector|MakeVector (.x _returnvalue) (.y _returnvalue) (.z _returnvalue))))
    (:then_3
      (Utilities|Time|SetTimerbyEvent (delegate Custom|PlayBearSound) (Math|Random|RandomFloatinRange 0.1 0.1)))))

(event EventTick
  (params (DeltaSeconds :type Float%20%28single-precision%29))
  (bind _returnvalue (Transformation|GetActorRotation))
  (bind _startlocation (Variables|Private|GetStartLocation))
  (Utilities|FlowControl|Sequence
    (:then_0
      (CallFunction|FloatonWater (Variables|Private|GetWaterSettings) (Variables|Private|GetInitialZ)))
    (:then_1
      (bind _output_get (Variables|Private|Set_currX (+ (* (Variables|Public|GetRadius) (Math|Trig|Sin(Degrees) (Variables|Private|Get_theta))) (.x _startlocation)))))
    (:then_2
      (if (Variables|Private|GetIsMovingLeft)
        (Variables|Private|Set_theta (+ (Variables|Private|Get_theta) (* -1 (Variables|Public|GetSpeed))))))
    (:then_3
      (if (Variables|Private|GetIsMovingRight)
        (Variables|Private|Set_theta (+ (Variables|Private|Get_theta) (Variables|Public|GetSpeed)))))
    (:then_4
      (bind _output_get_2 (Variables|Private|Set_currY (+ (* (Variables|Public|GetRadius) (Math|Trig|Cos(Degrees) (Variables|Private|Get_theta))) (.y _startlocation)))))
    (:then_5
      (Transformation|SetActorLocation (Math|Vector|MakeVector _output_get _output_get_2 (.z (Transformation|GetActorLocation))) false false))
    (:then_6
      (Transformation|SetWorldRotation (Variables|Collision|GetCapsuleComponent) (Math|Rotator|MakeRotator (.roll _returnvalue) (.pitch _returnvalue) (.yaw (Math|Rotator|FindLookatRotation (Transformation|GetWorldLocation (Variables|Collision|GetCapsuleComponent)) (Variables|Private|GetStartLocation)))) false false))
    (:then_7
      (bind _outhit (Collision|LineTraceByChannel (Transformation|GetActorLocation) (Variables|Private|GetStartLocation) "TraceTypeQuery1" false 0 "ForOneFrame"))
      (bind _asiceberg_chunk_1 (Utilities|Casting|CastToIceberg_chunk1 (Components|GetOwner (.hitcomponent _outhit))))
      (if (not (Variables|/Game/Blueprints/Iceberg_blueprints/Iceberg_chunk1.Iceberg_chunk1_C|GetIsChunkCaptured _asiceberg_chunk_1))
        (Variables|Default|SetTargetIcebergChunkComponent (.hitcomponent _outhit))
        (else
          (Variables|Default|SetTargetIcebergChunkComponent 0))))))

(event Input|ActionEvents|InputActionStaple
  (params (Key :type Key%20Structure))
  (:Pressed
    (CallFunction|ShootStaple)))

(event Input|ActionEvents|InputActionMoveLeft
  (params (Key :type Key%20Structure))
  ;[1 1 1] Character State / Input Handling
  (:Pressed
    (Variables|Private|SetIsMovingLeft true))
  (:Released
    (Variables|Private|SetIsMovingLeft false)))

(event Input|ActionEvents|InputActionMoveRight
  (params (Key :type Key%20Structure))
  ;[1 1 1] Character State / Input Handling
  (:Pressed
    (Variables|Private|SetIsMovingRight true))
  (:Released
    (Variables|Private|SetIsMovingRight false)))

(fn ConstructionScript)

(fn FloatonWater
  (params (WaterSettings :type Water%20Settings%20Object%20Reference) (InitialZ :type Float%20%28single-precision%29))
  (bind _returnvalue (Transformation|GetActorLocation))
  (Utilities|IsValid WaterSettings
    (:Is%20Valid
      (bind _delta (Default|CalculateDeltaOnly WaterSettings (Math|Vector2D|MakeVector2D (.x _returnvalue) (.y _returnvalue))))
      (Transformation|SetActorLocation (Math|Vector|MakeVector (.x _returnvalue) (.y _returnvalue) (+ (.z _delta) InitialZ)) false false))))

(fn IsIcebergChunk
  (params (TargetActor :type Actor%20Object%20Reference))
  (Utilities|Casting|CastToIceberg_chunk1 TargetActor
    (:then
      (LocalVariables|SetReturnValue true :!label _label))
    (:CastFailed
      (Utilities|Casting|CastToori_Iceberg_chunk2 TargetActor
        (:then
          (goto _label))
        (:CastFailed
          (Utilities|Casting|CastToIceberg_chunk3 TargetActor
            (:then
              (goto _label))
            (:CastFailed
              (LocalVariables|SetReturnValue false)))))))
  (return (LocalVariables|GetReturnValue)))

(fn PlayPaddleSounds
  (bind _audiocomponent (Variables|Default|GetAudioComponent))
  (bind _volumemultiplier (Variables|/Script/Engine.AudioComponent|GetVolumeMultiplier _audiocomponent))
  (switch int (Math|Random|RandomIntegerinRange 0 2)
    (:0
      (Audio|SpawnSoundAttached "/Game/Assets/Sound/SoundFX/Paddle_Left_1_Cue.Paddle_Left_1_Cue" _audiocomponent "None" "0, 0, 0" "0, 0, 0" "KeepRelativeOffset" false _volumemultiplier 1.0 0.0 0 0)
      (Audio|SpawnSoundAttached "/Game/Assets/Sound/SoundFX/Paddle_Right_1_Cue.Paddle_Right_1_Cue" _audiocomponent "None" "0, 0, 0" "0, 0, 0" "KeepRelativeOffset" false _volumemultiplier 1.0 0.0 0 0))
    (:1
      (Audio|SpawnSoundAttached "/Game/Assets/Sound/SoundFX/Paddle_Left_2_Cue.Paddle_Left_2_Cue" _audiocomponent "None" "0, 0, 0" "0, 0, 0" "KeepRelativeOffset" false _volumemultiplier 1.0 0.0 0 0)
      (Audio|SpawnSoundAttached "/Game/Assets/Sound/SoundFX/Paddle_Right_2_Cue.Paddle_Right_2_Cue" _audiocomponent "None" "0, 0, 0" "0, 0, 0" "KeepRelativeOffset" false _volumemultiplier 1.0 0.0 0 0))
    (:2
      (Audio|SpawnSoundAttached "/Game/Assets/Sound/SoundFX/Paddle_Left_3_Cue.Paddle_Left_3_Cue" _audiocomponent "None" "0, 0, 0" "0, 0, 0" "KeepRelativeOffset" false _volumemultiplier 1.0 0.0 0 0)
      (Audio|SpawnSoundAttached "/Game/Assets/Sound/SoundFX/Paddle_Right_3_Cue.Paddle_Right_3_Cue" _audiocomponent "None" "0, 0, 0" "0, 0, 0" "KeepRelativeOffset" false _volumemultiplier 1.0 0.0 0 0)))
  (return (Math|Random|RandomFloatinRange 0.3 5.0)))

(fn ShootStaple
  (bind _targeticebergchunkcomponent (Variables|Default|GetTargetIcebergChunkComponent))
  (Game|SpawnActorfromClass "/Game/Blueprints/Character/BP_StapleProjectile.BP_StapleProjectile_C" (Transformation|GetWorldTransform (Variables|Default|GetProjectileArrowComponent)) "Undefined" 0 0)
  (Audio|Components|Audio|Play (Variables|Default|GetStapleSound) 0.5)
  (Utilities|IsValid _targeticebergchunkcomponent
    (:Is%20Valid
      (bind _asiceberg_chunk_1 (Utilities|Casting|CastToIceberg_chunk1 (Components|GetOwner _targeticebergchunkcomponent)))
      (Variables|/Game/Blueprints/Iceberg_blueprints/Iceberg_chunk1.Iceberg_chunk1_C|SetIs%20chunk%20Stapled? _asiceberg_chunk_1 true)
      (Physics|AddImpulse (Variables|Default|GetTargetIcebergChunkComponent) (* (Math|Vector|GetForwardVector (Transformation|GetActorRotation)) (Variables|Public|GetImpulseStrength)) "None" true))))