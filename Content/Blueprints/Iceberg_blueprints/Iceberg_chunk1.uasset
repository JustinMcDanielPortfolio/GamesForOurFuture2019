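; An iceberg chunk actor that registers with its parent Iceberg and moves vertically with the water.
; Construction and BeginPlay apply the configurable mesh and material; BeginPlay also stores the starting Z, saves the index from registration and finds the first WaterSettings actor.
; Each Tick queries WaterSettings for a delta at its XY and adds that Z plus the initial Z onto its current location, so the offset is cumulative.
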(event EventBeginPlay
  (bind _returnvalue (Transformation|GetActorLocation))
  (CallFunction|SetupCustomMesh)
  (Variables|Default|SetStartLocation (Math|Vector|MakeVector (.x _returnvalue) (.y _returnvalue) (.z _returnvalue)))
  (Variables|Default|SetInitial%20Z (.z _returnvalue))
  (CallFunction|RegistertoParentIceberg)
  (bind _outactors (Actor|GetAllActorsOfClass "/Game/PhysicalWaterSurface/Blueprints/WaterSettings.WaterSettings_C"))
  (Variables|Default|SetWater%20Settings (Utilities|Array|Get(acopy) _outactors)))

(event EventTick
  (params (DeltaSeconds :type Float%20%28single-precision%29))
  (CallFunction|FloatonWater (Variables|Default|GetWater%20Settings) (Variables|Default|GetInitial%20Z)))

(fn ConstructionScript
  (CallFunction|SetupCustomMesh))

(fn FloatonWater
  (params (Water%20Settings :type Water%20Settings%20Object%20Reference) (Initial%20Z :type Float%20%28single-precision%29))
  (bind _returnvalue (Transformation|GetActorLocation))
  (Utilities|IsValid Water%20Settings
    (:Is%20Valid
      (bind _delta (Default|CalculateDeltaOnly Water%20Settings (Math|Vector2D|MakeVector2D (.x _returnvalue) (.y _returnvalue))))
      (Transformation|SetActorLocation (+ (Transformation|GetActorLocation) (Math|Vector|MakeVector 0.0 0.0 (+ (.z _delta) Initial%20Z))) false false))))

(fn RegistertoParentIceberg
  (bind _self self)
  (bind _returnvalue (Class|Actor|GetParentComponent _self))
  (bind _returnvalue_2 (Components|GetOwner _returnvalue))
  (bind _asiceberg (Utilities|Casting|CastToIceberg _returnvalue_2)
    (:then
      (bind _chunkindex (Default|RegisterIcebergChunk _asiceberg self))
      (Variables|Default|SetIcebergChunk%20Index _chunkindex))
    (:CastFailed
      (Development|PrintString (Utilities|GetDisplayName _returnvalue_2)))))

(fn SetupCustomMesh
  (bind _mesh (Variables|Default|GetMesh))
  (Components|StaticMesh|SetStaticMesh _mesh (Variables|MeshValues|GetDesiredMesh))
  (Rendering|Material|SetMaterial _mesh 0 (Variables|MeshValues|GetDesiredMaterial)))