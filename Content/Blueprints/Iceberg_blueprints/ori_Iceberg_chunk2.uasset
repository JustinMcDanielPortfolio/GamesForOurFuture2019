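; Iceberg chunk actor that bobs vertically on the water surface.
; BeginPlay records its starting Z and caches the first WaterSettings actor found in the level.
; Each Tick, FloatOnWater queries that actor's CalculateDeltaOnly at the chunk's XY and adds the Z delta to the starting height.
; It takes the new XY from IcebergChunkLocation, which this file never sets.
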(event EventBeginPlay
  (Variables|Default|SetInitial%20Z (.z (Transformation|GetActorLocation)))
  (bind _outactors (Actor|GetAllActorsOfClass "/Game/PhysicalWaterSurface/Blueprints/WaterSettings.WaterSettings_C"))
  (Variables|Default|SetWater%20Settings (Utilities|Array|Get(acopy) _outactors)))

(event Collision|EventActorBeginOverlap
  (params (OtherActor :type Actor%20Object%20Reference)))

(event EventTick
  (params (DeltaSeconds :type Float%20%28single-precision%29))
  (CallFunction|FloatonWater (Variables|Default|GetWater%20Settings) (Variables|Default|GetInitial%20Z)))

(fn ConstructionScript)

(fn FloatonWater
  (params (Water%20Settings :type Water%20Settings%20Object%20Reference) (Initial%20Z :type Float%20%28single-precision%29))
  (bind _returnvalue (Transformation|GetActorLocation))
  (bind _iceberg_chunk_location (Variables|Default|GetIceberg%20Chunk%20Location))
  (Utilities|IsValid Water%20Settings
    (:Is%20Valid
      (bind _delta (Default|CalculateDeltaOnly Water%20Settings (Math|Vector2D|MakeVector2D (.x _returnvalue) (.y _returnvalue))))
      (Transformation|SetActorLocationAndRotation (Math|Vector|MakeVector (.x _iceberg_chunk_location) (.y _iceberg_chunk_location) (+ (.z _delta) Initial%20Z)) "0, 0, 0"))))