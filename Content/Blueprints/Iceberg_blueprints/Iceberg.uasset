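; Iceberg actor that floats on the water, plays random bear sounds and periodically breaks off Iceberg_chunk1 pieces.
; A timer shoots a random attached chunk out with a radial impulse, on an arctangent-curved interval that shortens as the GameMode counter rises.
; Stapled chunks overlapping ChunkCollider snap back to their start XY and rejoin the ejection pool.
; Chunks leaving Bounds are removed and start dying.
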(event OnComponentEndOverlap(Bounds)
  (params (OverlappedComponent :type Primitive%20Component%20Object%20Reference) (OtherActor :type Actor%20Object%20Reference) (OtherComp :type Primitive%20Component%20Object%20Reference) (OtherBodyIndex :type Integer))
  (bind _asiceberg_chunk_1 (Utilities|Casting|CastToIceberg_chunk1 OtherActor))
  (Utilities|Array|RemoveItem (Variables|Default|GetIce_Chunks) _asiceberg_chunk_1)
  (Default|StartDying _asiceberg_chunk_1))

(event OnComponentBeginOverlap(ChunkCollider)
  (params (OverlappedComponent :type Primitive%20Component%20Object%20Reference) (OtherActor :type Actor%20Object%20Reference) (OtherComp :type Primitive%20Component%20Object%20Reference) (OtherBodyIndex :type Integer) (bFromSweep :type Boolean) (SweepResult :type Hit%20Result%20Structure%20%28by%20ref%29))
  (bind _asiceberg_chunk_1 (Utilities|Casting|CastToIceberg_chunk1 OtherActor))
  (CallFunction|AttachIceBacktoBerg _asiceberg_chunk_1))

(event Custom|Attach%20Ice%20back%20to%20Berg
  (params (Iceberg%20Chunk :type Iceberg%20Chunk%201%20Object%20Reference))
  (bind _startlocation (Variables|/Game/Blueprints/Iceberg_blueprints/Iceberg_chunk1.Iceberg_chunk1_C|GetStartLocation Iceberg%20Chunk))
  (if (Variables|/Game/Blueprints/Iceberg_blueprints/Iceberg_chunk1.Iceberg_chunk1_C|GetIs%20chunk%20Stapled? Iceberg%20Chunk)
    (Variables|/Game/Blueprints/Iceberg_blueprints/Iceberg_chunk1.Iceberg_chunk1_C|SetIsChunkCaptured Iceberg%20Chunk true)
    (Transformation|SetActorLocation Iceberg%20Chunk (Math|Vector|MakeVector (.x _startlocation) (.y _startlocation) (.z (Transformation|GetActorLocation Iceberg%20Chunk))) false false)
    (Physics|SetPhysicsLinearVelocity (Variables|/Game/Blueprints/Iceberg_blueprints/Iceberg_chunk1.Iceberg_chunk1_C|GetMesh Iceberg%20Chunk) "0, 0, 0" false "None")
    (Utilities|Array|Add (Variables|Default|GetIcebergChunkIndex) (Variables|/Game/Blueprints/Iceberg_blueprints/Iceberg_chunk1.Iceberg_chunk1_C|GetIcebergChunk%20Index Iceberg%20Chunk))))

(event Custom|Event%20Eject%20Iceberg
  (CallFunction|EjectIceberg)
  (Development|PrintString (Utilities|String|Append "Eject Iceberg in " (Utilities|String|ToString(Float) (Variables|Default|GetTime)) " Seconds") true true "(R=0.000000,G=0.660000,B=1.000000,A=1.000000)" 1.0)
  (bind _time (CallFunction|SetTime))
  (Utilities|Time|SetTimerbyEvent (delegate Custom|Event%20Eject%20Iceberg) _time))

(event Custom|PlayBearSound
  (bind _nexttime (CallFunction|PlayRoundSoundFX))
  (Utilities|Time|SetTimerbyEvent (delegate Custom|PlayBearSound) _nexttime))

(event EventBeginPlay
  (Utilities|Time|SetTimerbyEvent (delegate Custom|PlayBearSound) (Math|Random|RandomFloatinRange 0.3 5.0))
  (CallFunction|GetReferences)
  (if (and (Variables|Default|GetIs%20Time%20Greater%20Than%200?) (> (Variables|/Game/Blueprints/BP_GameMode.BP_GameMode_C|GetGlobal%20Time (Variables|Default|GetGameMode)) 0))
    (bind (_time _is_time_greater_than_0_) (CallFunction|SetTime))
    (Utilities|Time|SetTimerbyEvent (delegate Custom|Event%20Eject%20Iceberg) _time)
    (if _is_time_greater_than_0_
      (Variables|Default|SetIs%20Time%20Greater%20Than%200? true)
      (else
        (Variables|Default|SetIs%20Time%20Greater%20Than%200? false)))))

(event EventTick
  (params (DeltaSeconds :type Float%20%28single-precision%29))
  (CallFunction|FloatonWater (Variables|Default|GetWater%20Settings) (Variables|Default|GetInitial%20Z))
  (for _array_element (Variables|Default|GetIce_Chunks)
    (Utilities|IsValid _array_element
      (:Is%20Valid
        (Variables|/Game/Blueprints/Iceberg_blueprints/Iceberg_chunk1.Iceberg_chunk1_C|SetIceberg%20Chunk%20Location _array_element (Transformation|GetActorLocation _array_element))))))

(fn ConstructionScript)

(fn CreateArrayOfIcebergs
  (bind _outactors (Actor|GetAllActorsOfClass "/Game/Blueprints/Iceberg_blueprints/Iceberg_chunk1.Iceberg_chunk1_C"))
  (bind _output_get (Variables|Default|SetIce_Chunks _outactors))
  (for (_array_element _array_index) _output_get
    (bind _output_get_2 (Variables|/Game/Blueprints/Iceberg_blueprints/Iceberg_chunk1.Iceberg_chunk1_C|SetIcebergChunk%20Index _array_element _array_index))
    (Utilities|Array|Add (Variables|Default|GetIcebergChunkIndex) _output_get_2))
  (return))

(fn IcebergTimer
  (Variables|Default|Setx (+ (Variables|Default|Getx) 1))
  (bind _output_get (Variables|Default|SetTime%20Remaining (+ (* (Math|Float|Power 1.028 (Math|Conversions|ToFloat(Integer) (Variables|Default|Getx))) -1.0) 195.0)))
  (if (> (Variables|Default|GetTime%20Remaining) 0.0)
    (Variables|Default|SetIs%20Time%20Greater%20Than%200? true)
    (else
      (Variables|Default|SetIs%20Time%20Greater%20Than%200? false)))
  (Development|PrintString (Utilities|String|ToString(Integer) (Math|Float|Truncate _output_get)) true true "(R=0.000000,G=0.660000,B=1.000000,A=1.000000)" 1.0))

(fn EjectIceberg
  (Development|PrintString "Be gone Iceberg!" true true "(R=0.000000,G=0.660000,B=1.000000,A=1.000000)" 1.0)
  (Audio|Components|Audio|Play (Variables|Default|GetAudioIcebergCrack) 0.0)
  (bind _icebergchunk (CallFunction|GetIcebergPiece))
  (Physics|AddRadialImpulse (Variables|/Game/Blueprints/Iceberg_blueprints/Iceberg_chunk1.Iceberg_chunk1_C|GetMesh _icebergchunk) (Transformation|GetActorLocation) 2e+03 (Variables|IcebergSettings|GetEjectionVelocity) "RIF_Constant" true)
  (Variables|/Game/Blueprints/Iceberg_blueprints/Iceberg_chunk1.Iceberg_chunk1_C|SetIs%20chunk%20Stapled? _icebergchunk false)
  (Variables|/Game/Blueprints/Iceberg_blueprints/Iceberg_chunk1.Iceberg_chunk1_C|SetIsChunkCaptured _icebergchunk false))

(fn SetEjectTime
  (Variables|Default|Setx (+ (Variables|Default|Getx) 1))
  (bind _output_get (Variables|Default|SetEject%20Time (+ (* (Math|Trig|Atan(Degrees) (+ (* (Variables|Default|Getx) -0.1) 5.0)) 3.28) 5.5)))
  (Development|PrintString (Utilities|String|Append (Utilities|String|Append "eject time set to" (Utilities|String|ToString(Float) _output_get)) "seconds") true true "(R=0.000000,G=0.660000,B=1.000000,A=1.000000)" 1.0))

(fn SetTime
  (Variables|Default|Setx (Variables|/Game/Blueprints/BP_GameMode.BP_GameMode_C|GetGlobel%20Counter (Variables|Default|GetGameMode)))
  (bind _output_get (Variables|Default|SetTime (+ (* (Math|Trig|Atan(Degrees) (+ (* (Variables|Default|Getx) -0.1) 5.0)) 3.28) 5.5)))
  (Development|PrintString (Utilities|String|Append (Utilities|String|Append "Eject Iceberg in " (Utilities|String|ToString(Float) _output_get)) " seconds") true true "(R=0.000000,G=0.660000,B=1.000000,A=1.000000)" 1.0)
  (return (Variables|Default|GetTime) (> (Variables|Default|GetTime) 0.0)))

(fn IsGameStillPlaying
  (params (Is%20Time%20Greater%20than%200? :type Boolean))
  (bind _output_get (Variables|Default|SetIs%20Game%20Still%20Playing? Is%20Time%20Greater%20than%200?))
  (return _output_get))

(fn GetIcebergPiece
  (bind _icebergchunkindex (Variables|Default|GetIcebergChunkIndex))
  (Utilities|Array|Shuffle _icebergchunkindex)
  (LocalVariables|SetReturn%20Value (Utilities|Array|Get(acopy) (Variables|Default|GetIce_Chunks) (Utilities|Array|Get(acopy) _icebergchunkindex)))
  (Utilities|Array|RemoveIndex _icebergchunkindex)
  (return (LocalVariables|GetReturn%20Value)))

(fn FloatonWater
  (params (Water%20Settings :type Water%20Settings%20Object%20Reference) (Initial%20Z :type Float%20%28single-precision%29))
  (bind _returnvalue (Transformation|GetActorLocation))
  (Utilities|IsValid Water%20Settings
    (:Is%20Valid
      (bind _delta (Default|CalculateDeltaOnly Water%20Settings (Math|Vector2D|MakeVector2D (.x _returnvalue) (.y _returnvalue))))
      (Transformation|SetActorLocation (Math|Vector|MakeVector (.x _returnvalue) (.y _returnvalue) (+ (.z _delta) Initial%20Z)) false false))))

(fn PlayRoundSoundFX
  (bind _audiocomponent (Variables|Default|GetAudioComponent))
  (bind _soundfx (Variables|Default|GetSoundFX))
  (bind _returnvalue (Utilities|Array|Length _soundfx))
  (if (> _returnvalue 0)
    (Audio|SpawnSoundAttached (Utilities|Array|Get(acopy) (Variables|Default|GetSoundFX) (Math|Random|RandomIntegerinRange 0 (- _returnvalue 1))) _audiocomponent "None" "0, 0, 0" "0, 0, 0" "KeepRelativeOffset" false (Variables|/Script/Engine.AudioComponent|GetVolumeMultiplier _audiocomponent) 1.0 0.0 0 0)
    (return (Math|Random|RandomFloatinRange 0.3 5.0))))

(fn GetReferences
  (Variables|Default|SetInitial%20Z (.z (Transformation|GetActorLocation)))
  (bind _outactors (Actor|GetAllActorsOfClass "/Game/Blueprints/Timer.Timer_C"))
  (bind _output_get (Variables|Default|SetTimer%20Class _outactors))
  (Variables|Default|SetTimer (Utilities|Array|Get(acopy) _output_get))
  (bind _outactors_2 (Actor|GetAllActorsOfClass "/Game/Blueprints/BP_GameMode.BP_GameMode_C"))
  (Variables|Default|SetGameMode (Utilities|Array|Get(acopy) _outactors_2))
  (bind _outactors_3 (Actor|GetAllActorsOfClass "/Game/PhysicalWaterSurface/Blueprints/WaterSettings.WaterSettings_C"))
  (Variables|Default|SetWater%20Settings (Utilities|Array|Get(acopy) _outactors_3)))

(fn RegisterIcebergChunk
  (params (IcebergChunk :type Iceberg%20Chunk%201%20Object%20Reference))
  (bind _returnvalue (Utilities|Array|Add (Variables|Default|GetIce_Chunks) IcebergChunk))
  (Utilities|Array|Add (Variables|Default|GetIcebergChunkIndex) _returnvalue)
  (return _returnvalue))